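; Player controller for the Paladin character that owns the player's on-screen HUD.
; On BeginPlay it creates the PlayerUI widget, adds it to the viewport and keeps a reference.
; SetHUDParameters reads Health, Stamina and Fury from BP_PlayerState and passes each to the widget as a fraction of its maximum.
; A disconnected branch that would update the pawn's healthbar widget never runs.
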(event EventBeginPlay
  (bind _returnvalue (UserInterface|CreateWidget "/Game/TrialOfMight/UI/PlayerUI.PlayerUI_C"))
  (UserInterface|Viewport|AddtoViewport _returnvalue 0)
  (Variables|Default|SetPlayerUI _returnvalue))

(event EventTick
  (params (DeltaSeconds :type Float%20%28single-precision%29)))

(fn ConstructionScript)

(fn SetHUDParameters
  (bind _asbp_player_state (Utilities|Casting|CastToBP_PlayerState (Variables|GetPlayerState)))
  (Default|SetHUDParameters (Variables|Default|GetPlayerUI) (/ (Variables|/Game/TrialOfMight/Characters/Paladin/BP_PlayerState.BP_PlayerState_C|GetHealth _asbp_player_state) (Variables|/Game/TrialOfMight/Characters/Paladin/BP_PlayerState.BP_PlayerState_C|GetMaxHealth _asbp_player_state)) (/ (Variables|/Game/TrialOfMight/Characters/Paladin/BP_PlayerState.BP_PlayerState_C|GetStamina _asbp_player_state) (Variables|/Game/TrialOfMight/Characters/Paladin/BP_PlayerState.BP_PlayerState_C|GetMaxStamina _asbp_player_state)) (/ (Variables|/Game/TrialOfMight/Characters/Paladin/BP_PlayerState.BP_PlayerState_C|GetFury _asbp_player_state) (Variables|/Game/TrialOfMight/Characters/Paladin/BP_PlayerState.BP_PlayerState_C|GetMaxFury _asbp_player_state))))