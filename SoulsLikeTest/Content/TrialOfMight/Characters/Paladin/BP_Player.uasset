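; Player character for melee combat, with lock-on to another BP_Player, directional rolls, light/heavy attacks and weapon pickup/drop.
; Inputs route through Event/All wrappers to montage playback, using "ComboOpened" sections to chain attacks.
; Attack inputs pick up overlapping BP_Weapons when unarmed; WeaponHit passes damage to the held weapon.
; Tick polls montages to freeze movement during light attacks and pickup, disable capsule overlaps during rolls, and updates roll direction.
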(event Custom|Drop%20Weapon%20Event
  (CallFunction|DropWeaponEventAll))

(event Custom|Drop%20Weapon%20Event%20All
  (CallFunction|DropWeapon))

(event Custom|Set%20Roll%20Direction
  ;[1 1 1] Set Roll Direction SPAGHETTI MONSTER
  (if (< (stale Input|AxisEvents|InputAxisHorizontal AxisValue) 0.0)
    (Variables|Default|SetRollDirection "NewEnumerator0")
    (elif (> (stale Input|AxisEvents|InputAxisHorizontal AxisValue) 0.0)
      (Variables|Default|SetRollDirection "NewEnumerator2")
      (elif (< (stale Input|AxisEvents|InputAxisVertical AxisValue) 0.0)
        (Variables|Default|SetRollDirection "NewEnumerator3")
        (else
          (Variables|Default|SetRollDirection "NewEnumerator1"))))))

(event Custom|Light%20Attack%20Event
  (CallFunction|LightAttackEventAll))

(event Custom|Heavy%20Attack%20Event
  (CallFunction|HeavyAttackEventAll))

(event Custom|Weapon%20Hit
  (Default|DamagePlayer (Variables|Default|GetRightWeapon)))

(event Custom|Target%20Set
  (bind _hastarget (Variables|Default|GetHasTarget))
  ;[1 1 1] Look at opponent while targeting
  (Variables|Default|SetbUseControllerRotationYaw self _hastarget)
  (if _hastarget
    (Variables|Default|SetSpeedMultiplier (Variables|Default|GetWalkingSpeedMultiplier))
    (else
      (Variables|Default|SetSpeedMultiplier (Variables|Default|GetRunningSpeedMultiplier)))))

(event Custom|Roll%20Event%20All
  ;[1 1 1] If no other animations are playing
  (if (not (Animation|Montage|MontageIsPlaying (Components|SkeletalMesh|GetAnimInstance (Variables|Character|GetMesh)) 0))
    ;[1 1 1] If Player is targeting
    (if (Variables|Default|GetHasTarget)
      (switch Utilities|FlowControl|Switch|SwitchonE_Direction (Variables|Default|GetRollDirection)
        (:NewEnumerator0
          ;[1 1 1] Do Left Roll
          (Animation|Montage|MontagePlay (Variables|Default|GetAnimation) "/Game/TrialOfMight/Characters/Paladin/Montages/AM_LeftRoll.AM_LeftRoll" 1.0 "MontageLength" 0.0 true))
        (:NewEnumerator1
          ;[1 1 1] Do Forward Roll
          (Animation|Montage|MontagePlay (Variables|Default|GetAnimation) "/Game/TrialOfMight/Characters/Paladin/Montages/AM_Roll.AM_Roll" 1.0 "MontageLength" 0.0 true :!label _label))
        (:NewEnumerator2
          ;[1 1 1] Do Right Roll
          (Animation|Montage|MontagePlay (Variables|Default|GetAnimation) "/Game/TrialOfMight/Characters/Paladin/Montages/AM_RightRoll.AM_RightRoll" 1.0 "MontageLength" 0.0 true))
        (:NewEnumerator3
          ;[1 1 1] Do Back Dash
          (Animation|Montage|MontagePlay (Variables|Default|GetAnimation) "/Game/TrialOfMight/Characters/Paladin/Montages/AM_BackDash.AM_BackDash" 1.0 "MontageLength" 0.0 true :!label _label_2)))
      (else
        ;[1 1 1] If Player is not moving
        (if (< (Math|Vector|VectorLength (Transformation|GetVelocity)) 0.2)
          (goto _label_2)
          (else
            (goto _label)))))))

(event Custom|Roll%20Event
  (CallFunction|RollEventAll))

(event Custom|Init%20Animation
  (Variables|Default|SetAnimation (Components|SkeletalMesh|GetAnimInstance (Variables|Character|GetMesh))))

(event Custom|Light%20Attack%20Event%20All
  (bind _mesh (Variables|Character|GetMesh))
  (bind _returnvalue (Components|SkeletalMesh|GetAnimInstance _mesh))
  (bind _returnvalue_2 (CallFunction|PlayerHasWeaponEquipped))
  (if _returnvalue_2
    ;[1 1 1] If is playing light attack 1
    (if (Utilities|Name|Equal(Name) (Animation|Montage|MontageGetCurrentSection _returnvalue "/Game/TrialOfMight/Characters/Paladin/Montages/AM_LightAttack1.AM_LightAttack1") "ComboOpened")
      ;[1 1 1] Do Light Attack 2
      (Animation|Montage|MontagePlay (Variables|Default|GetAnimation) "/Game/TrialOfMight/Characters/Paladin/Montages/AM_LightAttack2.AM_LightAttack2" 1.0 "MontageLength" 0.0 true)
      (else
        ;[1 1 1] If is playing light attack 2
        (if (Utilities|Name|Equal(Name) (Animation|Montage|MontageGetCurrentSection _returnvalue "/Game/TrialOfMight/Characters/Paladin/Montages/AM_LightAttack2.AM_LightAttack2") "ComboOpened")
          ;[1 1 1] Do Light Attack
          (Animation|Montage|MontagePlay (Variables|Default|GetAnimation) "/Game/TrialOfMight/Characters/Paladin/Montages/AM_LightAttack1.AM_LightAttack1" 1.0 "MontageLength" 0.0 true :!label _label)
          (else
            ;[1 1 1] If the animation is playing
            (if (not (Animation|Montage|MontageIsPlaying _returnvalue 0))
              (goto _label))))))
    (else
      (CallFunction|CheckGroundandPickWeapon))))

(event Custom|Heavy%20Attack%20Event%20All
  (bind _mesh (Variables|Character|GetMesh))
  (bind _returnvalue (Components|SkeletalMesh|GetAnimInstance _mesh))
  (bind _returnvalue_2 (CallFunction|PlayerHasWeaponEquipped))
  (if _returnvalue_2
    ;[1 1 1] If is light attacking
    (if (or (Utilities|Name|Equal(Name) (Animation|Montage|MontageGetCurrentSection _returnvalue "/Game/TrialOfMight/Characters/Paladin/Montages/AM_LightAttack1.AM_LightAttack1") "ComboOpened") (Utilities|Name|Equal(Name) (Animation|Montage|MontageGetCurrentSection _returnvalue "/Game/TrialOfMight/Characters/Paladin/Montages/AM_LightAttack2.AM_LightAttack2") "ComboOpened"))
      ;[1 1 1] Do heavy attack
      (Animation|Montage|MontagePlay (Variables|Default|GetAnimation) "/Game/TrialOfMight/Characters/Paladin/Montages/AM_HeavyAttack.AM_HeavyAttack" 1.0 "MontageLength" 0.0 true :!label _label)
      (else
        ;[1 1 1] If the animation is playing
        (if (not (Animation|Montage|MontageIsPlaying _returnvalue 0))
          (goto _label))))
    (else
      (CallFunction|CheckGroundandPickWeapon))))

(event EventTick
  (params (DeltaSeconds :type Float%20%28single-precision%29))
  (bind _charactermovement (Variables|Character|GetCharacterMovement))
  (bind _mesh (Variables|Character|GetMesh))
  (bind _capsulecomponent (Variables|Collision|GetCapsuleComponent))
  (bind _returnvalue (Components|SkeletalMesh|GetAnimInstance _mesh))
  (Utilities|FlowControl|Sequence
    (:then_0
      (if (Animation|Montage|MontageIsPlaying _returnvalue "/Game/TrialOfMight/Characters/Paladin/Montages/AM_LightAttack1.AM_LightAttack1")
        (Pawn|Components|CharacterMovement|SetMovementMode _charactermovement "MOVE_None" 0 :!label _label)
        (elif (Animation|Montage|MontageIsPlaying _returnvalue "/Game/TrialOfMight/Characters/Paladin/Montages/AM_LightAttack2.AM_LightAttack2")
          (goto _label)
          (elif (Animation|Montage|MontageIsPlaying _returnvalue "/Game/TrialOfMight/Characters/Paladin/Montages/AM_WeaponPick.AM_WeaponPick")
            (goto _label)
            (else
              (Pawn|Components|CharacterMovement|SetMovementMode _charactermovement "MOVE_Walking" 0))))))
    (:then_1
      (if (Animation|Montage|MontageIsPlaying _returnvalue "/Game/TrialOfMight/Characters/Paladin/Montages/AM_Roll.AM_Roll")
        (Variables|/Script/Engine.PrimitiveComponent|SetbGenerateOverlapEvents _capsulecomponent false :!label _label_2)
        (elif (Animation|Montage|MontageIsPlaying _returnvalue "/Game/TrialOfMight/Characters/Paladin/Montages/AM_LeftRoll.AM_LeftRoll")
          (goto _label_2)
          (elif (Animation|Montage|MontageIsPlaying _returnvalue "/Game/TrialOfMight/Characters/Paladin/Montages/AM_RightRoll.AM_RightRoll")
            (goto _label_2)
            (else
              (Variables|/Script/Engine.PrimitiveComponent|SetbGenerateOverlapEvents _capsulecomponent true))))))
    (:then_2
      (CallFunction|SetRollDirection))))

(event EventBeginPlay
  (Utilities|FlowControl|Sequence
    (:then_0
      (CallFunction|InitAnimation))
    (:then_1
      (CallFunction|TargetSet))))

(event Input|ActionEvents|InputActionRoll
  (params (Key :type Key%20Structure))
  (:Pressed
    (CallFunction|RollEvent)))

(event Input|ActionEvents|InputActionHeavyAttack
  (params (Key :type Key%20Structure))
  (:Pressed
    (CallFunction|HeavyAttackEvent)))

(event Input|ActionEvents|InputActionTarget
  (params (Key :type Key%20Structure))
  (bind _returnvalue (Pawn|GetController))
  (bind _returnvalue_2 (Pawn|GetControlRotation _returnvalue :!class /Script/Engine.Controller))
  (bind (_roll _pitch) (Math|Rotator|BreakRotator _returnvalue_2))
  ;[1 1 1] Targeting
  (:Pressed
    (if (Variables|Default|GetHasTarget)
      (Variables|Default|SetHasTarget false)
      (CallFunction|TargetSet)
      (goto _label Toggle)
      (else
        (bind _outactors (Actor|GetAllActorsOfClass "BP_Player_C"))
        (for _array_element _outactors
          (Timeline|Timeline_0 Play
            (:Update
              (Utilities|FlowControl|Gate true :!label _label
                (:Exit
                  (Pawn|SetControlRotation _returnvalue (Math|Rotator|MakeRotator _roll _pitch (.Yaw (Math|Rotator|BreakRotator (Math|Interpolation|RInterpTo _returnvalue_2 (Math|Rotator|FindLookatRotation (Transformation|GetWorldLocation (Variables|Default|GetCamera)) (Transformation|GetActorLocation (Variables|Default|GetTarget))) (Utilities|Time|GetWorldDeltaSeconds) 7.0))))))))))
        (Variables|Default|SetHasTarget true)
        (CallFunction|TargetSet)
        (Variables|Default|SetTarget _array_element)
        (Utilities|FlowControl|Gate true) ; enters at Toggle
      ))))

(event Input|ActionEvents|InputActionDropWeapon
  (params (Key :type Key%20Structure))
  (:Pressed
    (CallFunction|DropWeaponEvent)))

(event Input|ActionEvents|InputActionLightAttack
  (params (Key :type Key%20Structure))
  (:Pressed
    (CallFunction|LightAttackEvent)))

(event Input|AxisEvents|InputAxisHorizontal
  (params (AxisValue :type Float%20%28single-precision%29))
  ;[1 1 1] Character Movement
  (Pawn|Input|AddMovementInput (Math|Vector|GetRightVector (Math|Rotator|MakeRotator 0.0 0.0 (.Yaw (Math|Rotator|BreakRotator (Pawn|GetControlRotation :!class /Script/Engine.Pawn))))) (* AxisValue (Variables|Default|GetSpeedMultiplier)) false))

(event Input|AxisEvents|InputAxisVertical
  (params (AxisValue :type Float%20%28single-precision%29))
  ;[1 1 1] Character Movement
  (Pawn|Input|AddMovementInput (Math|Vector|GetForwardVector (Math|Rotator|MakeRotator 0.0 0.0 (.Yaw (Math|Rotator|BreakRotator (Pawn|GetControlRotation :!class /Script/Engine.Pawn))))) (* AxisValue (Variables|Default|GetSpeedMultiplier)) false))

(event Input|AxisEvents|InputAxisCameraPitch
  (params (AxisValue :type Float%20%28single-precision%29))
  ;[1 1 1] Camera Stuff
  (Pawn|Input|AddControllerPitchInput (* (* (Variables|Default|GetCameraRotationSpeed) (Utilities|Time|GetWorldDeltaSeconds)) AxisValue)))

(event Input|AxisEvents|InputAxisHorizontal
  (params (AxisValue :type Float%20%28single-precision%29))
  ;[1 1 1] Set Roll Direction SPAGHETTI MONSTER
)

(event Input|AxisEvents|InputAxisVertical
  (params (AxisValue :type Float%20%28single-precision%29))
  ;[1 1 1] Set Roll Direction SPAGHETTI MONSTER
)

(event Input|AxisEvents|InputAxisCameraYaw
  (params (AxisValue :type Float%20%28single-precision%29))
  ;[1 1 1] Camera Stuff
  (Pawn|Input|AddControllerYawInput (* (* (Variables|Default|GetCameraRotationSpeed) (Utilities|Time|GetWorldDeltaSeconds)) AxisValue)))

(fn ConstructionScript)

(fn IsWeapon
  (params (Object :type Object%20Object%20Reference))
  (return (Utilities|ClassIsChildOf (Utilities|GetClass Object) "/Game/TrialOfMight/Weapons/BP_Weapon.BP_Weapon_C")))

(fn PlayerHasWeaponEquipped
  (return (Utilities|IsValid (Variables|Default|GetRightWeapon))))

(fn DropWeapon
  (bind _self self)
  (bind _returnvalue (CallFunction|PlayerHasWeaponEquipped))
  (if _returnvalue
    (Transformation|DetachFromActor (Variables|Default|GetRightWeapon) "KeepRelative" "KeepRelative" "KeepRelative")
    (Transformation|SetActorLocation (Variables|Default|GetRightWeapon) (+ (Transformation|GetActorLocation _self) (* (Transformation|GetActorForwardVector _self) 3e+02)) false false)
    (Default|Unequip (Variables|Default|GetRightWeapon))
    (Variables|Default|SetRightWeapon 0)))

(fn PickWeapon
  (params (Collision :type Actor%20Object%20Reference))
  (bind _returnvalue (CallFunction|IsWeapon Collision))
  (bind _asbp_weapon (Utilities|Casting|CastToBP_Weapon Collision))
  (if _returnvalue
    (bind _returnvalue_2 (CallFunction|PlayerHasWeaponEquipped))
    (if _returnvalue_2
      (if (CallFunction|CheckifWeaponIsEquipped _asbp_weapon)
        (CallFunction|DropWeapon))
      (else
        (Transformation|AttachComponentToComponent Collision (Variables|Character|GetMesh) "RightWeapon" "SnapToTarget" "SnapToTarget" "SnapToTarget" false)
        (bind _output_get (Variables|Default|SetRightWeapon _asbp_weapon))
        (Default|Equip _output_get self)))))

(fn CheckifWeaponIsEquipped
  (params (Weapon :type BP%20Weapon%20Object%20Reference))
  (return (== (Variables|Default|GetRightWeapon) Weapon)))

(fn CheckGroundandPickWeapon
  (bind _capsulecomponent (Variables|Collision|GetCapsuleComponent))
  (bind _overlappingactors (Collision|GetOverlappingActors _capsulecomponent "/Game/TrialOfMight/Weapons/BP_Weapon.BP_Weapon_C" :!class /Script/Engine.PrimitiveComponent))
  (if (> (Utilities|Array|Length _overlappingactors) 0)
    (Animation|PlayAnimMontage "/Game/TrialOfMight/Characters/Paladin/Montages/AM_WeaponPick.AM_WeaponPick" 1.0 "None")
    (CallFunction|PickWeapon (Utilities|Array|Get(acopy) _overlappingactors))))