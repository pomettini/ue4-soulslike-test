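; Equippable weapon actor with its own health, shown on a healthbar widget.
; Equip and Unequip track the holding player; DoDamage checks the mesh for overlapping BP_Player actors other than the holder.
; Each hit calls DamagePlayer, which despite its name subtracts fixed health from the weapon itself, not the player struck.
; Health changes refresh the bar and, at zero, trigger the weapon's destroy event chain.
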(event Custom|Equip
  (params (Owner :type BP%20Player%20Object%20Reference))
  (Variables|Default|SetEquippedPlayer Owner)
  (Rendering|SetVisibility (Variables|Default|GetWidget) true false))

(event Custom|Destroy%20Weapon%20Event
  (CallFunction|DestroyWeaponEventAll))

(event Custom|CheckCollision
  (if (CallFunction|IsEquipped)
    (for _array_element (Collision|GetOverlappingActors (Variables|Default|GetStaticMesh) "/Game/TrialOfMight/Characters/Paladin/BP_Player.BP_Player_C" :!class /Script/Engine.PrimitiveComponent)
      (if (!= _array_element (Variables|Default|GetEquippedPlayer))
        (CallFunction|DamagePlayer)))))

(event Custom|Destroy%20Weapon%20Event%20All
  (Actor|DestroyActor))

(event Custom|DamagePlayer
  (CallFunction|DecreaseHealth 2e+01))

(event Custom|Unequip
  (Variables|Default|SetEquippedPlayer 0)
  (Rendering|SetVisibility (Variables|Default|GetWidget) true false))

(event Custom|DoDamage
  (CallFunction|CheckCollision))

(event EventBeginPlay
  (CallFunction|UpdateHealth))

(fn ConstructionScript
  (Variables|Default|SetHealth (Variables|Default|GetMaxHealth)))

(fn IsEquipped
  (return (Utilities|IsValid (Variables|Default|GetEquippedPlayer))))

(fn DecreaseHealth
  (params (Amount :type Float%20%28single-precision%29))
  (Variables|Default|SetHealth (- (Variables|Default|GetHealth) Amount))
  (CallFunction|UpdateHealth))

(fn UpdateHealth
  (bind _maxhealth (Variables|Default|GetMaxHealth))
  (bind _health (Variables|Default|GetHealth))
  (bind _returnvalue (/ _health _maxhealth))
  (bind _ashealthbar_widget (Utilities|Casting|CastToHealthbarWidget (UserInterface|GetUserWidgetObject (Variables|Default|GetWidget))))
  (Default|SetHealthPercentage _ashealthbar_widget _returnvalue)
  (if (<= _returnvalue 0.0)
    (CallFunction|DestroyWeaponEvent)))