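; BP_Paladin is a Souls-like playable character with camera-relative movement, target lock-on, rolls and melee attacks.
; Lock-on picks from other BP_Paladin actors, switches speed and yaw control, and uses a timeline-fed gate to turn toward the target.
; Actions pass through Event/All wrappers to montages, with "ComboOpened" sections chaining attacks and Tick freezing movement during light attacks.
; DoDamage briefly enables sword overlaps, and any foreign capsule overlap destroys the character.
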(event OnComponentBeginOverlap(CapsuleComponent)
  (params (OverlappedComponent :type Primitive%20Component%20Object%20Reference) (OtherActor :type Actor%20Object%20Reference) (OtherComp :type Primitive%20Component%20Object%20Reference) (OtherBodyIndex :type Integer) (bFromSweep :type Boolean) (SweepResult :type Hit%20Result%20Structure%20%28by%20ref%29))
  (if (!= OtherActor self)
    (CallFunction|GetDamagedEvent)))

(event Custom|Do%20Damage
  (bind _swordtrigger (Variables|Default|GetSwordTrigger))
  (Variables|/Script/Engine.PrimitiveComponent|SetbGenerateOverlapEvents _swordtrigger true)
  (Utilities|FlowControl|Delay 0.1)
  (Variables|/Script/Engine.PrimitiveComponent|SetbGenerateOverlapEvents _swordtrigger false))

(event Custom|Light%20Attack%20Event
  (CallFunction|LightAttackEventAll))

(event Custom|Heavy%20Attack%20Event
  (CallFunction|HeavyAttackEventAll))

(event Custom|Target%20Set
  (bind _hastarget (Variables|Default|GetHasTarget))
  (Variables|Default|SetbUseControllerRotationYaw self _hastarget)
  (if _hastarget
    (Variables|Default|SetSpeedMultiplier (Variables|Default|GetWalkingSpeedMultiplier))
    (else
      (Variables|Default|SetSpeedMultiplier (Variables|Default|GetRunningSpeedMultiplier)))))

(event Custom|Roll%20Event%20All
  (bind _mesh (Variables|Character|GetMesh))
  (bind _returnvalue (Components|SkeletalMesh|GetAnimInstance _mesh))
  ;[1 1 1] If no other animations are playing
  (if (not (Animation|Montage|MontageIsPlaying _returnvalue 0))
    ;[1 1 1] If Player is not moving
    (if (< (Math|Vector|VectorLength (Transformation|GetVelocity)) 0.1)
      ;[1 1 1] If Player is targeting
      (if true
        (switch Utilities|FlowControl|Switch|SwitchonE_Direction "NewEnumerator0")
        (else
          ;[1 1 1] Do Back Dash
          (Animation|Montage|MontagePlay _returnvalue "/Game/SoulsLike/Characters/Paladin/Montages/AM_BackDash.AM_BackDash" 1.0 "MontageLength" 0.0)))
      (else
        ;[1 1 1] Do Roll
        (Animation|Montage|MontagePlay _returnvalue "/Game/SoulsLike/Characters/Paladin/Montages/AM_Roll.AM_Roll" 1.0 "MontageLength" 0.0)))))

(event Custom|Roll%20Event
  (CallFunction|RollEventAll))

(event Custom|Get%20Damaged%20Event
  (CallFunction|GetDamagedEventAll))

(event Custom|Light%20Attack%20Event%20All
  (bind _mesh (Variables|Character|GetMesh))
  (bind _returnvalue (Components|SkeletalMesh|GetAnimInstance _mesh))
  ;[1 1 1] If is playing light attack 1
  (if (Utilities|Name|Equal(Name) (Animation|Montage|MontageGetCurrentSection _returnvalue "/Game/SoulsLike/Characters/Paladin/Montages/AM_LightAttack1.AM_LightAttack1") "ComboOpened")
    ;[1 1 1] Do Light Attack 2
    (Animation|Montage|MontagePlay _returnvalue "/Game/SoulsLike/Characters/Paladin/Montages/AM_LightAttack2.AM_LightAttack2" 1.0 "MontageLength" 0.0)
    (else
      ;[1 1 1] If is playing light attack 2
      (if (Utilities|Name|Equal(Name) (Animation|Montage|MontageGetCurrentSection _returnvalue "/Game/SoulsLike/Characters/Paladin/Montages/AM_LightAttack2.AM_LightAttack2") "ComboOpened")
        ;[1 1 1] Do Light Attack
        (Animation|Montage|MontagePlay _returnvalue "/Game/SoulsLike/Characters/Paladin/Montages/AM_LightAttack1.AM_LightAttack1" 1.0 "MontageLength" 0.0 :!label _label)
        (else
          ;[1 1 1] If the animation is playing
          (if (not (Animation|Montage|MontageIsPlaying _returnvalue 0))
            (goto _label)))))))

(event Custom|Get%20Damaged%20Event%20All
  (Actor|DestroyActor))

(event Custom|Heavy%20Attack%20Event%20All
  (bind _mesh (Variables|Character|GetMesh))
  (bind _returnvalue (Components|SkeletalMesh|GetAnimInstance _mesh))
  ;[1 1 1] If is light attacking
  (if (or (Utilities|Name|Equal(Name) (Animation|Montage|MontageGetCurrentSection _returnvalue "/Game/SoulsLike/Characters/Paladin/Montages/AM_LightAttack1.AM_LightAttack1") "ComboOpened") (Utilities|Name|Equal(Name) (Animation|Montage|MontageGetCurrentSection _returnvalue "/Game/SoulsLike/Characters/Paladin/Montages/AM_LightAttack2.AM_LightAttack2") "ComboOpened"))
    ;[1 1 1] Do heavy attack
    (Animation|Montage|MontagePlay _returnvalue "/Game/SoulsLike/Characters/Paladin/Montages/AM_HeavyAttack.AM_HeavyAttack" 1.0 "MontageLength" 0.0 :!label _label)
    (else
      ;[1 1 1] If the animation is playing
      (if (not (Animation|Montage|MontageIsPlaying _returnvalue 0))
        (goto _label)))))

(event EventTick
  (params (DeltaSeconds :type Float%20%28single-precision%29))
  (bind _charactermovement (Variables|Character|GetCharacterMovement))
  (bind _mesh (Variables|Character|GetMesh))
  (bind _returnvalue (Components|SkeletalMesh|GetAnimInstance _mesh))
  (if (Animation|Montage|MontageIsPlaying _returnvalue "/Game/SoulsLike/Characters/Paladin/Montages/AM_LightAttack1.AM_LightAttack1")
    (Pawn|Components|CharacterMovement|SetMovementMode _charactermovement "MOVE_None" 0 :!label _label)
    (elif (Animation|Montage|MontageIsPlaying _returnvalue "/Game/SoulsLike/Characters/Paladin/Montages/AM_LightAttack2.AM_LightAttack2")
      (goto _label)
      (else
        (Pawn|Components|CharacterMovement|SetMovementMode _charactermovement "MOVE_Walking" 0)))))

(event EventBeginPlay
  (Variables|/Script/Engine.PrimitiveComponent|SetbGenerateOverlapEvents (Variables|Default|GetSwordTrigger) false)
  (CallFunction|TargetSet))

(event Input|ActionEvents|InputActionRoll
  (params (Key :type Key%20Structure))
  (:Pressed
    (CallFunction|RollEvent)))

(event Input|ActionEvents|InputActionHeavyAttack
  (params (Key :type Key%20Structure))
  (:Pressed
    (CallFunction|HeavyAttackEvent)))

(event Input|ActionEvents|InputActionTarget
  (params (Key :type Key%20Structure))
  (bind _returnvalue (Pawn|GetController))
  (bind _returnvalue_2 (Pawn|GetControlRotation _returnvalue :!class /Script/Engine.Controller))
  (bind (_roll _pitch) (Math|Rotator|BreakRotator _returnvalue_2))
  (:Pressed
    (if (Variables|Default|GetHasTarget)
      (Variables|Default|SetHasTarget false)
      (CallFunction|TargetSet)
      (goto _label Toggle)
      (else
        (bind _outactors (Actor|GetAllActorsOfClass "BP_Paladin_C"))
        (for _array_element _outactors
          (Timeline|Timeline_0 Play
            (:Update
              (Utilities|FlowControl|Gate true :!label _label
                (:Exit
                  (Pawn|SetControlRotation _returnvalue (Math|Rotator|MakeRotator _roll _pitch (.Yaw (Math|Rotator|BreakRotator (Math|Interpolation|RInterpTo _returnvalue_2 (Math|Rotator|FindLookatRotation (Transformation|GetWorldLocation (Variables|Default|GetCamera)) (Transformation|GetActorLocation (Variables|Default|GetTarget))) (Utilities|Time|GetWorldDeltaSeconds) 7.0))))))))))
        (Variables|Default|SetHasTarget true)
        (CallFunction|TargetSet)
        (Variables|Default|SetTarget _array_element)
        (Utilities|FlowControl|Gate true) ; enters at Toggle
      ))))

(event Input|ActionEvents|InputActionLightAttack
  (params (Key :type Key%20Structure))
  (:Pressed
    (CallFunction|LightAttackEvent)))

(event Input|AxisEvents|InputAxisHorizontal
  (params (AxisValue :type Float%20%28single-precision%29))
  ;[1 1 1] Character Movement
  (Pawn|Input|AddMovementInput (Math|Vector|GetRightVector (Math|Rotator|MakeRotator 0.0 0.0 (.Yaw (Math|Rotator|BreakRotator (Pawn|GetControlRotation :!class /Script/Engine.Pawn))))) (* AxisValue (Variables|Default|GetSpeedMultiplier)) false))

(event Input|AxisEvents|InputAxisVertical
  (params (AxisValue :type Float%20%28single-precision%29))
  ;[1 1 1] Character Movement
  (Pawn|Input|AddMovementInput (Math|Vector|GetForwardVector (Math|Rotator|MakeRotator 0.0 0.0 (.Yaw (Math|Rotator|BreakRotator (Pawn|GetControlRotation :!class /Script/Engine.Pawn))))) (* AxisValue (Variables|Default|GetSpeedMultiplier)) false))

(event Input|AxisEvents|InputAxisCameraPitch
  (params (AxisValue :type Float%20%28single-precision%29))
  ;[1 1 1] Camera Stuff
  (Pawn|Input|AddControllerPitchInput (* (* (Variables|Default|GetCameraRotationSpeed) (Utilities|Time|GetWorldDeltaSeconds)) AxisValue)))

(event Input|AxisEvents|InputAxisCameraYaw
  (params (AxisValue :type Float%20%28single-precision%29))
  ;[1 1 1] Camera Stuff
  (Pawn|Input|AddControllerYawInput (* (* (Variables|Default|GetCameraRotationSpeed) (Utilities|Time|GetWorldDeltaSeconds)) AxisValue)))

(fn ConstructionScript)