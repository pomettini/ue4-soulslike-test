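; BP_Weapon is a weapon Blueprint for a souls-like game that tracks which player has it equipped.
; Equip and Unequip set or clear that player reference, and both make its widget visible.
; Every tick it polls the mesh for overlapping BP_Paladin actors, printing a debug "Hello" on screen for any other than the wielder.
; DamagePlayer is an empty stub, and construction initializes Health from MaxHealth.
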(event Custom|Equip
  (params (Owner :type BP%20Paladin%20Object%20Reference))
  (Variables|Default|SetEquippedPlayer Owner)
  (Rendering|SetVisibility (Variables|Default|GetWidget) true false))

(event Custom|CheckCollision
  (for _array_element (Collision|GetOverlappingActors (Variables|Default|GetStaticMesh) "/Game/SoulsLike/Characters/Paladin/BP_Paladin.BP_Paladin_C" :!class /Script/Engine.PrimitiveComponent)
    (Development|PrintString "Hello" (!= _array_element (Variables|Default|GetEquippedPlayer)))))

(event Custom|DamagePlayer)

(event Custom|Unequip
  (Variables|Default|SetEquippedPlayer 0)
  (Rendering|SetVisibility (Variables|Default|GetWidget) true false))

(event EventTick
  (params (DeltaSeconds :type Float%20%28single-precision%29))
  (CallFunction|CheckCollision))

(fn ConstructionScript
  (Variables|Default|SetHealth (Variables|Default|GetMaxHealth)))

(fn IsEquipped
  (return (Utilities|IsValid (Variables|Default|GetEquippedPlayer))))